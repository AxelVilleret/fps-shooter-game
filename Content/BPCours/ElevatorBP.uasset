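; Elevator actor that rises when the first-person player steps into its trigger box, provided all detected enemies are killed.
; The kill check compares the player's NumberOfKills, read from the character found on BeginPlay, with NumberOfDetectedEnnemies in the custom game instance.
; A timeline drives the elevator's relative Z location on entry and reverses when the player leaves the box.
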(event OnComponentBeginOverlap(Box)
  (params (OverlappedComponent :type Primitive%20Component%20Object%20Reference) (OtherActor :type Actor%20Object%20Reference) (OtherComp :type Primitive%20Component%20Object%20Reference) (OtherBodyIndex :type Integer) (bFromSweep :type Boolean) (SweepResult :type Hit%20Result%20Structure%20%28by%20ref%29))
  (Utilities|Casting|CastToFirstPersonCharacter OtherActor)
  (bind _returnvalue (CallFunction|HasPlayerKilledAllEnnemies))
  (if _returnvalue
    (bind _zvalue (Timeline|Elevator_T Play)
      (:Update
        (Transformation|SetRelativeLocation (Variables|Default|GetElevator) (Math|Vector|MakeVector 0.0 0.0 (* _zvalue 1e+03)) false false)))))

(event OnComponentEndOverlap(Box)
  (params (OverlappedComponent :type Primitive%20Component%20Object%20Reference) (OtherActor :type Actor%20Object%20Reference) (OtherComp :type Primitive%20Component%20Object%20Reference) (OtherBodyIndex :type Integer))
  (Utilities|Casting|CastToFirstPersonCharacter OtherActor)
  (bind _zvalue (Timeline|Elevator_T Reverse)
    (:Update
      (Transformation|SetRelativeLocation (Variables|Default|GetElevator) (Math|Vector|MakeVector 0.0 0.0 (* _zvalue 1e+03)) false false))))

(event EventBeginPlay
  (bind _outactors (Actor|GetAllActorsOfClass "/Game/FirstPersonBP/Blueprints/FirstPersonCharacter.FirstPersonCharacter_C"))
  (Variables|Default|Setplayer (.OutItem (Utilities|Array|Random _outactors))))

(fn ConstructionScript)

(fn HasPlayerKilledAllEnnemies
  (bind _ascustom_game_instance_bp (Utilities|Casting|CastToCustomGameInstanceBP (Game|GetGameInstance)))
  (return (== (Variables|/Game/FirstPersonBP/Blueprints/FirstPersonCharacter.FirstPersonCharacter_C|GetnumberOfKills (Variables|Default|Getplayer)) (Variables|/Game/FirstPersonBP/Blueprints/CustomGameInstanceBP.CustomGameInstanceBP_C|GetNumberOfDetectedEnnemies _ascustom_game_instance_bp))))