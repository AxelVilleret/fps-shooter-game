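; Base enemy character that wanders randomly, chases the player when seen within detection range or shot, and attacks on overlap.
; Walk, detect, run and hit functions form a state machine gated by allowed-previous-state lists, each setting speed, animation and sound.
; Looping timers drive wandering and damage to the player.
; Projectile hits drain a health widget; death destroys the enemy, increments player kills and grants a secret code on the first.
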(event OnSeePawn(PawnSensing)
  (params (Pawn :type Pawn%20Object%20Reference))
  (if (not (Variables|Default|GetisDead))
    (if (== Pawn (Game|Player|GetPlayerPawn 0))
      (bind _isplayerdetected (CallFunction|IsPlayerDetected))
      (if _isplayerdetected
        (CallFunction|Detect)
        (Utilities|FlowControl|Delay (Variables|/Script/Engine.AnimSequenceBase|GetSequenceLength (Variables|Default|GetdetectionAnimation)))
        (CallFunction|Run)
        (AI|AIMoveTo self "0, 0, 0" (Game|Player|GetPlayerPawn 0) 5.0 true)))))

(event OnComponentHit(Box)
  (params (HitComponent :type Primitive%20Component%20Object%20Reference) (OtherActor :type Actor%20Object%20Reference) (OtherComp :type Primitive%20Component%20Object%20Reference) (NormalImpulse :type Vector :default "0, 0, 0") (Hit :type Hit%20Result%20Structure%20%28by%20ref%29))
  (if (not (Variables|Default|GetisDead))
    (Utilities|Casting|CastToFirstPersonProjectile OtherActor)
    (CallFunction|LoseLife)
    (if (<= (Variables|Default|GetennemyLife) 0.0)
      (CallFunction|Dead)
      (Utilities|FlowControl|Delay (Variables|/Script/Engine.AnimSequenceBase|GetSequenceLength (Variables|Default|GetdeathAnimation)))
      (Actor|DestroyActor)
      (bind _asfirst_person_character (Utilities|Casting|CastToFirstPersonCharacter (Variables|Default|Getplayer)))
      (bind _output_get (Variables|/Game/FirstPersonBP/Blueprints/FirstPersonCharacter.FirstPersonCharacter_C|SetnumberOfKills _asfirst_person_character (+ (Variables|/Game/FirstPersonBP/Blueprints/FirstPersonCharacter.FirstPersonCharacter_C|GetnumberOfKills _asfirst_person_character) 1)))
      (Math|Integer|CompareInt _output_get 1
        (:==
          (Variables|/Game/FirstPersonBP/Blueprints/FirstPersonCharacter.FirstPersonCharacter_C|SetsecretCode _asfirst_person_character "1234")))
      (else
        (CallFunction|OnDammageReceived)))))

(event Custom|onDammageReceived
  (CallFunction|Detect)
  (Utilities|FlowControl|Delay (Variables|/Script/Engine.AnimSequenceBase|GetSequenceLength (Variables|Default|GetdetectionAnimation)))
  (CallFunction|Run)
  (AI|AIMoveTo self "0, 0, 0" (Game|Player|GetPlayerPawn 0) 5.0 true))

(event EventBeginPlay
  (CallFunction|Walk)
  (Utilities|Time|SetTimerbyFunctionName 0 "moveRandomly" 2.0 true)
  (bind _outactors (Actor|GetAllActorsOfClass "/Game/FirstPersonBP/Blueprints/FirstPersonCharacter.FirstPersonCharacter_C"))
  (Variables|Default|Setplayer (.OutItem (Utilities|Array|Random _outactors))))

(event Collision|EventActorBeginOverlap
  (params (OtherActor :type Actor%20Object%20Reference))
  (Utilities|Casting|CastToFirstPersonCharacter OtherActor)
  (CallFunction|Hit)
  (bind _returnvalue (Utilities|Time|SetTimerbyFunctionName 0 "losePlayerLife" (Variables|/Script/Engine.AnimSequenceBase|GetSequenceLength (Variables|Default|GethitAnimation)) true))
  (Variables|Default|SetisAttacking _returnvalue))

(event Collision|EventActorEndOverlap
  (params (OtherActor :type Actor%20Object%20Reference))
  (Utilities|Casting|CastToFirstPersonCharacter OtherActor)
  (CallFunction|Walk)
  (Utilities|Time|ClearandInvalidateTimerbyHandle (Variables|Default|GetisAttacking)))

(fn ConstructionScript)

(fn LoseLife
  (Variables|Default|SetennemyLife (Math|Float|SelectFloat (- (Variables|Default|GetennemyLife) 5.0) 0.0 (> (- (Variables|Default|GetennemyLife) 5.0) 0.0)))
  (bind _aslife (Utilities|Casting|CastToLife (UserInterface|GetUserWidgetObject (Variables|Default|GetWidget))))
  (Variables|/Game/Ennemy/Widgets/Life.Life_C|Sethealth _aslife (/ (Variables|Default|GetennemyLife) (Variables|Default|GetmaxLife)))
  (return))

(fn MoveRandomly
  (if (not (Variables|Default|GetisPlayerVisible))
    (AI|Navigation|SimpleMovetoLocation (Pawn|GetController) (.RandomLocation (AI|Navigation|GetRandomReachablePointinRadius (Transformation|GetActorLocation) 1e+03 0 0)))
    (return)))

(fn Walk
  (bind _istransitionnauthorized (CallFunction|IsTranstionAuthorized "walk"))
  (if _istransitionnauthorized
    (Variables|Default|SetcurrentState "walk")
    (Variables|Default|SetisPlayerVisible false)
    (Variables|/Script/Engine.CharacterMovementComponent|SetMaxWalkSpeed (Variables|Character|GetCharacterMovement) (Variables|Default|GetwalkSpeed))
    (Components|Animation|PlayAnimation (Variables|Character|GetMesh) (Variables|Default|GetwalkAnimation) true)
    (CallFunction|PlaySound (Variables|Default|GetwalkSound))
    (return)))

(fn Run
  (bind _istransitionnauthorized (CallFunction|IsTranstionAuthorized "run"))
  (if _istransitionnauthorized
    (Variables|Default|SetcurrentState "run")
    (Variables|/Script/Engine.CharacterMovementComponent|SetMaxWalkSpeed (Variables|Character|GetCharacterMovement) (Variables|Default|GetrunSpeed))
    (Components|Animation|PlayAnimation (Variables|Character|GetMesh) (Variables|Default|GetrunAnimation) true)
    (CallFunction|PlaySound (Variables|Default|GetrunSound))
    (return)))

(fn Hit
  (bind _istransitionnauthorized (CallFunction|IsTranstionAuthorized "hit"))
  (if _istransitionnauthorized
    (Variables|Default|SetcurrentState "hit")
    (Variables|/Script/Engine.CharacterMovementComponent|SetMaxWalkSpeed (Variables|Character|GetCharacterMovement) 0.0)
    (Components|Animation|PlayAnimation (Variables|Character|GetMesh) (Variables|Default|GethitAnimation) true)
    (CallFunction|PlaySound (Variables|Default|GethitSound))
    (return)))

(fn IsTranstionAuthorized
  (params (nextState :type String))
  (switch string nextState
    (:hit
      (LocalVariables|SetisTransitionAuthorized (Utilities|Array|ContainsItem (Variables|Default|GetauthorizedPreviousStatesHit) (Variables|Default|GetcurrentState))))
    (:walk
      (LocalVariables|SetisTransitionAuthorized (Utilities|Array|ContainsItem (Variables|Default|GetauthorizedPreviousStatesWalk) (Variables|Default|GetcurrentState))))
    (:run
      (LocalVariables|SetisTransitionAuthorized (Utilities|Array|ContainsItem (Variables|Default|GetauthorizedPreviousStatesRun) (Variables|Default|GetcurrentState))))
    (:detect
      (LocalVariables|SetisTransitionAuthorized (Utilities|Array|ContainsItem (Variables|Default|GetauthorizedPreviousStatesDetect) (Variables|Default|GetcurrentState)))))
  (return (LocalVariables|GetisTransitionAuthorized)))

(fn PlaySound
  (params (sound :type Sound%20Base%20Object%20Reference))
  (if (== (Variables|Default|GetCurrentSound) 0)
    _
    (else
      (Audio|Components|Audio|Stop (Variables|Default|GetCurrentSound))))
  (bind _returnvalue (Audio|SpawnSoundAttached sound (Variables|Default|GetBox) "None" (Transformation|GetActorLocation) "0, 0, 0" "KeepRelativeOffset" false 1.0 1.0 0.0 0 0))
  (Variables|Default|SetCurrentSound _returnvalue)
  (return))

(fn LosePlayerLife
  (bind _asfirst_person_character (Utilities|Casting|CastToFirstPersonCharacter (Game|GetPlayerCharacter 0)))
  (Default|LoseLife _asfirst_person_character)
  (return))

(fn IsPlayerDetected
  (return (<= (Transformation|GetDistanceTo self (Game|GetPlayerCharacter 0)) (Variables|Default|GetdetectionDistance))))

(fn Detect
  (bind _istransitionnauthorized (CallFunction|IsTranstionAuthorized "detect"))
  (if _istransitionnauthorized
    (Variables|Default|SetcurrentState "detect")
    (Variables|Default|SetisPlayerVisible true)
    (Variables|/Script/Engine.CharacterMovementComponent|SetMaxWalkSpeed (Variables|Character|GetCharacterMovement) 0.0)
    (Components|Animation|PlayAnimation (Variables|Character|GetMesh) (Variables|Default|GetdetectionAnimation) true)
    (CallFunction|PlaySound (Variables|Default|GetdetectionSound))
    (return)))

(fn Dead
  (Variables|Default|SetisDead true)
  (Variables|/Script/Engine.CharacterMovementComponent|SetMaxWalkSpeed (Variables|Character|GetCharacterMovement) 0.0)
  (Components|Animation|PlayAnimation (Variables|Character|GetMesh) (Variables|Default|GetdeathAnimation) false)
  (CallFunction|PlaySound (Variables|Default|GetdeathSound)))