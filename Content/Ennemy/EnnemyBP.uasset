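; Enemy character that wanders, chases the player on sight within range, drains their life while overlapping, and respawns a copy where it died.
; A string state machine with allowed-previous-state lists gates Walk, Run and Hit, each setting speed, animation and sound.
; Looping timers drive random wandering and attack damage, while PawnSensing triggers the chase.
; Projectile hits on the Box lower health and its widget bar, leading to death, destruction and respawn.
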(event OnSeePawn(PawnSensing)
  (params (Pawn :type Pawn%20Object%20Reference))
  (if (not (Variables|Default|GetisDead))
    (if (== Pawn (Game|Player|GetPlayerPawn 0))
      (bind _isplayerdetected (CallFunction|IsPlayerDetected))
      (if _isplayerdetected
        (CallFunction|Run)
        (AI|AIMoveTo self "0, 0, 0" (Game|Player|GetPlayerPawn 0) 5.0 true)))))

(event OnComponentHit(Box)
  (params (HitComponent :type Primitive%20Component%20Object%20Reference) (OtherActor :type Actor%20Object%20Reference) (OtherComp :type Primitive%20Component%20Object%20Reference) (NormalImpulse :type Vector :default "0, 0, 0") (Hit :type Hit%20Result%20Structure%20%28by%20ref%29))
  (bind _self self)
  (bind _returnvalue (Transformation|GetActorLocation _self))
  (if (not (Variables|Default|GetisDead))
    (Utilities|Casting|CastToFirstPersonProjectile OtherActor)
    (CallFunction|LoseLife)
    (if (<= (Variables|Default|GetennemyLife) 0.0)
      (bind _output_get (Variables|Default|SetspawnTransform _returnvalue))
      (Variables|Default|SetisDead true)
      (Components|Movement|StopMovementImmediately (Variables|Character|GetCharacterMovement))
      (Components|Animation|PlayAnimation (Variables|Character|GetMesh) "/Game/AnimStarterPack/Death_3.Death_3" false)
      (CallFunction|PlaySound "/Game/Sounds/death.death")
      (Audio|PlaySoundatLocation "/Game/Sounds/death-2.death-2" _returnvalue "0, 0, 0" 1.0 1.0 0.0 0 0 0)
      (Utilities|FlowControl|Delay 2.0)
      (Actor|DestroyActor)
      (bind _returnvalue_2 (Game|SpawnActorfromClass "EnnemyBP_C" (Math|Transform|MakeTransform _output_get "0, 0, 0" "1,1,1") "Undefined" 0 0))
      (Class|PawnSensingComponent|SetSensingUpdatesEnabled (Variables|EnnemyBP_C|GetPawnSensing _returnvalue_2) true))))

(event EventBeginPlay
  (CallFunction|Walk)
  (Utilities|Time|SetTimerbyFunctionName 0 "moveRandomly" 2.0 true))

(event Collision|EventActorBeginOverlap
  (params (OtherActor :type Actor%20Object%20Reference))
  (Utilities|Casting|CastToFirstPersonCharacter OtherActor)
  (CallFunction|Hit)
  (bind _returnvalue (Utilities|Time|SetTimerbyFunctionName 0 "losePlayerLife" 1.0 true))
  (Variables|Default|SetisAttacking _returnvalue))

(event Collision|EventActorEndOverlap
  (params (OtherActor :type Actor%20Object%20Reference))
  (Utilities|Casting|CastToFirstPersonCharacter OtherActor)
  (CallFunction|Walk)
  (Utilities|Time|ClearandInvalidateTimerbyHandle (Variables|Default|GetisAttacking)))

(fn ConstructionScript)

(fn LoseLife
  (Variables|Default|SetennemyLife (Math|Float|SelectFloat (- (Variables|Default|GetennemyLife) 5.0) 0.0 (> (- (Variables|Default|GetennemyLife) 5.0) 0.0)))
  (bind _asennemy_life (Utilities|Casting|CastToEnnemyLife (UserInterface|GetUserWidgetObject (Variables|Default|GetWidget))))
  (Variables|/Game/Ennemy/EnnemyLife.EnnemyLife_C|Sethealth _asennemy_life (/ (Variables|Default|GetennemyLife) (Variables|Default|GetmaxLife)))
  (return))

(fn MoveRandomly
  (if (not (Variables|Default|GetisPlayerVisible))
    (AI|Navigation|SimpleMovetoLocation (Pawn|GetController) (.RandomLocation (AI|Navigation|GetRandomReachablePointinRadius (Transformation|GetActorLocation) 1e+03 0 0)))
    (return)))

(fn Walk
  (bind _istransitionnauthorized (CallFunction|IsTranstionAuthorized "walk"))
  (if _istransitionnauthorized
    (Variables|Default|SetcurrentState "walk")
    (Variables|Default|SetisPlayerVisible false)
    (Variables|/Script/Engine.CharacterMovementComponent|SetMaxWalkSpeed (Variables|Character|GetCharacterMovement) 175.0)
    (Components|Animation|PlayAnimation (Variables|Character|GetMesh) "/Game/Ennemy/WalkAnim.WalkAnim" true)
    (CallFunction|PlaySound "/Game/Sounds/walk_cue.walk_cue")
    (return)))

(fn Run
  (bind _istransitionnauthorized (CallFunction|IsTranstionAuthorized "run"))
  (if _istransitionnauthorized
    (Variables|Default|SetcurrentState "run")
    (Variables|Default|SetisPlayerVisible true)
    (Audio|PlaySoundatLocation "/Game/Sounds/enemy-detected.enemy-detected" (Transformation|GetActorLocation) "0, 0, 0" 1.0 1.0 0.0 0 0 0)
    (Variables|/Script/Engine.CharacterMovementComponent|SetMaxWalkSpeed (Variables|Character|GetCharacterMovement) 6e+02)
    (Components|Animation|PlayAnimation (Variables|Character|GetMesh) "/Game/AnimStarterPack/Sprint_Fwd_Rifle.Sprint_Fwd_Rifle" true)
    (CallFunction|PlaySound "/Game/Sounds/run_cue.run_cue")
    (return)))

(fn Hit
  (bind _istransitionnauthorized (CallFunction|IsTranstionAuthorized "hit"))
  (if _istransitionnauthorized
    (Variables|Default|SetcurrentState "hit")
    (Variables|/Script/Engine.CharacterMovementComponent|SetMaxWalkSpeed (Variables|Character|GetCharacterMovement) 0.0)
    (Components|Animation|PlayAnimation (Variables|Character|GetMesh) "/Game/AnimStarterPack/Fire_Rifle_Ironsights.Fire_Rifle_Ironsights" true)
    (CallFunction|PlaySound "/Game/Sounds/hit_cue.hit_cue")
    (return)))

(fn IsTranstionAuthorized
  (params (nextState :type String))
  (switch string nextState
    (:hit
      (LocalVariables|SetisTransitionAuthorized (Utilities|Array|ContainsItem (Variables|Default|GetauthorizedPreviousStatesHit) (Variables|Default|GetcurrentState))))
    (:walk
      (LocalVariables|SetisTransitionAuthorized (Utilities|Array|ContainsItem (Variables|Default|GetauthorizedPreviousStatesWalk) (Variables|Default|GetcurrentState))))
    (:run
      (LocalVariables|SetisTransitionAuthorized (Utilities|Array|ContainsItem (Variables|Default|GetauthorizedPreviousStatesRun) (Variables|Default|GetcurrentState)))))
  (return (LocalVariables|GetisTransitionAuthorized)))

(fn PlaySound
  (params (sound :type Sound%20Base%20Object%20Reference))
  (if (== (Variables|Default|GetCurrentSound) 0)
    _
    (else
      (Audio|Components|Audio|Stop (Variables|Default|GetCurrentSound))))
  (bind _returnvalue (Audio|SpawnSoundAttached sound (Variables|Default|GetBox) "None" (Transformation|GetActorLocation) "0, 0, 0" "KeepRelativeOffset" false 1.0 1.0 0.0 0 0))
  (Variables|Default|SetCurrentSound _returnvalue)
  (return))

(fn LosePlayerLife
  (bind _asfirst_person_character (Utilities|Casting|CastToFirstPersonCharacter (Game|GetPlayerCharacter 0)))
  (Default|LoseLife _asfirst_person_character)
  (return))

(fn IsPlayerDetected
  (return (<= (Transformation|GetDistanceTo self (Game|GetPlayerCharacter 0)) 1e+03)))